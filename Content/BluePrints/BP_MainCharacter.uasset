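; Main character Blueprint that lets the player click world-space widgets and can detect a music player in view.
; The 1 key presses and releases the left mouse button through a WidgetInteraction component, with a debug print on press.
; A separate function line-traces forward from the camera and prints when the hit actor is a MusicPlayer.
; Nothing in these graphs calls that trace, and Tick and BeginPlay are empty.
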(event `self.ReceiveTick`
  (params (DeltaSeconds :type "Float (single-precision)")))

(event `Key|One`
  (params (Key :type "Key Structure"))
  (bind _widgetinteraction (`self.WidgetInteraction`))
  (:`Pressed`
    (`KismetSystemLibrary.PrintString` "1")
    (`WidgetInteractionComponent.PressPointerKey` _widgetinteraction "LeftMouseButton"))
  (:`Released`
    (`WidgetInteractionComponent.ReleasePointerKey` _widgetinteraction "LeftMouseButton")))

(fn `LineTraceforMusicPlayer`
  (bind _cameracomponent (`self.CameraComponent`))
  (bind _returnvalue (`SceneComponent.K2_GetComponentLocation` _cameracomponent))
  (bind (_outhit _returnvalue_2) (`KismetSystemLibrary.LineTraceSingle` _returnvalue (+ _returnvalue (* (`KismetMathLibrary.GetForwardVector` (`SceneComponent.K2_GetComponentRotation` _cameracomponent)) 10000.0)) "TraceTypeQuery3"))
  (if _returnvalue_2
    (cast `/Game/BluePrints/MusicPlayer` (`ActorComponent.GetOwner` (`.HitComponent` (`GameplayStatics.BreakHitResult` _outhit))))
    (`KismetSystemLibrary.PrintString` "Find Player")))

(fn `UserConstructionScript`)