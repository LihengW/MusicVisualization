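; Audio-reactive microphone receiver actor with switchable capture, driving a sphere material, Niagara particles and an optional ground-traced 3D spectrum.
; Tick averages submix frequency magnitudes over a sample window into the material's amplitude, while MetaSound peak output sets particle MusicAmp.
; An attraction sphere is added at startup, and up to two wind-target actors steer the center particles.
; A widget billboards toward the player camera; the burst-spawn branch is disconnected.
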(event `self.ReceiveBeginPlay`
  (bind _centerparticles (`self.CenterParticles`))
  (bind _returnvalue (`SceneComponent.K2_GetComponentLocation` _centerparticles))
  (`|ExecutionSequence`
    (:`then_1`
      (set `self.MaterialParameters` "/Game/Materials/AudioParameters.AudioParameters")
      (for _index (range (+ (`KismetArrayLibrary.Array_Length` (`self.searchfreqs`)) 1))
        (`KismetArrayLibrary.Array_Insert` (`self.nummemoarray`) 0 _index)
        (`KismetArrayLibrary.Array_Insert` (`self.memoarray`) 0.0 _index)
        (`KismetArrayLibrary.Array_Insert` (`self.PastValueArray`) 0.0 _index)))
    (:`then_2`
      ;[1 1 1] Init Spectrum (if use)
      (if (`self.spectrumOn`)
        (bind (_success _particlesystem) (`self.CreateSpectrum`))
        (if _success
          (set `self.CoreSpectrumSystem` _particlesystem))))
    (:`then_3`
      ;[1 1 1] Attraction Sphere Collision Spawn
      (bind _returnvalue_2 (`AddComponent|NODE_AddSphereComponent-0`))
      (`SphereComponent.SetSphereRadius` _returnvalue_2 (`self.AttractionRadius`) false)
      (`PrimitiveComponent.SetCollisionProfileName` _returnvalue_2 "AttractionDetection" true)
      (`SceneComponent.K2_AttachToComponent` _returnvalue_2 (`self.Sphere`) "None" "KeepRelative" "KeepRelative" "KeepRelative" true)
      (set `self.WindDetectionSphere` _returnvalue_2))
    (:`then_4`
      ;[1 1 1] Init Niagara Parameters for CenterParticles
      (`NiagaraComponent.SetVariableVec3` _centerparticles "WindTarget1" _returnvalue)
      (`NiagaraComponent.SetVariableVec3` _centerparticles "WindTarget2" _returnvalue))))

(event `self.ReceiveTick`
  (params (DeltaSeconds :type "Float (single-precision)"))
  (bind _widget (`self.Widget`))
  (bind _hasspectrum (`self.HasSpectrum`))
  (bind _centerparticles (`self.CenterParticles`))
  (bind _windtargeactorarray (`self.WindTargeActorArray`))
  (bind _returnvalue (`KismetArrayLibrary.Array_Length` _windtargeactorarray))
  (bind _returnvalue_2 (`SceneComponent.K2_GetComponentLocation` (`self.Sphere`)))
  (`|ExecutionSequence`
    (:`then_0`
      ;[1 1 1] Spectrum Generation Update
      (if (`self.spectrumOn`)
        (if _hasspectrum
          (if (`self.Moved`)
            (`ActorComponent.K2_DestroyComponent` (`self.CoreSpectrumSystem`))
            (bind (_success _particlesystem) (`self.CreateSpectrum`))
            (if _success
              (set `self.CoreSpectrumSystem` _particlesystem)
              (set `self.HasSpectrum` true)
              (set `self.Moved` false)
              (else
                (`KismetSystemLibrary.PrintString` "Spectrum Create Unsuccessfully!"))))
          (else
            (bind (_success_2 _particlesystem_2) (`self.CreateSpectrum`))
            (if _success_2
              (set `self.CoreSpectrumSystem` _particlesystem_2)
              (set `self.HasSpectrum` true)
              (else
                (`KismetSystemLibrary.PrintString` "Spectrum Create Unsuccessfully!")))))
        (elif _hasspectrum
          (`ActorComponent.K2_DestroyComponent` (`self.CoreSpectrumSystem`))
          (set `self.CoreSpectrumSystem` null)
          (set `self.HasSpectrum` false))))
    (:`then_1`
      ;[1 1 1] Monitor the output from meta sound output
      (`MetaSoundOutputSubsystem.WatchOutput` (subsystem `MetaSoundOutputSubsystem`) null "PeakOutput" (delegate `ReceiveOutputChange`) "None" "None"))
    (:`then_2`
      (bind _magnitudes (`AudioMixerBlueprintLibrary.GetMagnitudeForFrequencies` (`|MakeArray` 2000.0 4000.0 10000.0 :!type "Float (single-precision)") (`self.AudioSubmix`)))
      (for (_array_element _array_index) _magnitudes
        (bind (_value _output) (`self.Smooth Value` (`KismetMathLibrary.MultiplyMultiply_FloatFloat` (`KismetMathLibrary.FClamp` _array_element 0.0 1000.0) 0.3) _array_index))
        (if _output
          (`MeshComponent.SetScalarParameterValueOnMaterials` (`self.SphereMesh`) "audioamp" _value)
          (bind _output_2 (`|GetArrayItem` (`self.PastValueArray`) _array_index))
          (if (not (>= (- _value _output_2) (`self.BurstEdge`)))
            (`|VariableSetRef` _output_2 _value)))))
    (:`then_3`
      ;[1 1 1] Update Wind Target Position
      (if (>= _returnvalue 1)
        (`NiagaraComponent.SetVariableVec3` _centerparticles "WindTarget1" (`SceneComponent.K2_GetComponentLocation` (`/Game/BluePrints/MusicPlayer.Sphere` (`|GetArrayItem` _windtargeactorarray))))
        (if (>= _returnvalue 2)
          (`NiagaraComponent.SetVariableVec3` _centerparticles "WindTarget2" (`SceneComponent.K2_GetComponentLocation` (`/Game/BluePrints/MusicPlayer.Sphere` (`|GetArrayItem` _windtargeactorarray 1)))))))
    (:`then_4`
      ;[1 1 1] Widget Update
      (bind _asbp_main_character (cast `/Game/BluePrints/BP_MainCharacter` (`GameplayStatics.GetPlayerPawn` 0)))
      (bind _returnvalue_3 (- (`SceneComponent.K2_GetComponentLocation` (`MainCharacter.CameraComponent` _asbp_main_character)) _returnvalue_2))
      (`SceneComponent.K2_SetWorldRotation` _widget (`KismetMathLibrary.MakeRotFromX` _returnvalue_3) false false)
      (`SceneComponent.K2_SetWorldLocation` _widget (+ _returnvalue_2 (* (`KismetMathLibrary.Normal` _returnvalue_3) 400.0)) false false))))

(event `ReceiveOutputChange`
  (params (OutputName :type Name) (Output :type "MetaSoundOutput Structure (by ref)"))
  ;[1 1 1] Monitor the output from meta sound output
  (bind (_success _returnvalue) (`MetasoundOutputBlueprintAccess.GetFloat` Output))
  (if _success
    (`NiagaraComponent.SetVariableFloat` (`self.CenterParticles`) "MusicAmp" _returnvalue)))

(fn `CreateSpectrum`
  (returns (Success :type Boolean) (ParticleSystem :type "NiagaraComponent Object Reference"))
  (bind _returnvalue (`SceneComponent.K2_GetComponentLocation` (`self.SphereMesh`)))
  (if (`self.HasSpectrum`)
    (`KismetSystemLibrary.PrintString` "Already have a Spectrum")
    (else
      (bind _outhit (`KismetSystemLibrary.LineTraceSingle` _returnvalue (+ _returnvalue (* (`KismetMathLibrary.Vector_Down`) 1000.0)) "TraceTypeQuery1" true))
      (bind (_bblockinghit _binitialoverlap _time _distance _location) (`GameplayStatics.BreakHitResult` _outhit))
      (if _bblockinghit
        (bind _returnvalue_2 (`NiagaraFunctionLibrary.SpawnSystemAtLocation` "/Game/Niagara/3DshapeSpectrum.3DshapeSpectrum" _location))
        (`NiagaraComponent.SetVariableLinearColor` _returnvalue_2 "ColorHighV" (`KismetMathLibrary.Conv_VectorToLinearColor` (`self.mainColor`)))
        (`NiagaraComponent.SetVariableLinearColor` _returnvalue_2 "ColorLowV" (`KismetMathLibrary.Conv_VectorToLinearColor` (`self.SubColor`)))
        (set `self.HasSpectrum` true)
        (return _bblockinghit _returnvalue_2)
        (else
          (`KismetSystemLibrary.PrintString` "Don't Hit Surface"))))))

(fn `EndListenning`
  (locals (RecordingString :type String :default "Recording"))
  (`SynthComponent.Stop` (`self.AudioCaptureComp`))
  (set `self.Listenning` false))

(fn `Smooth Value`
  (params (accvalue :type "Float (double-precision)") (channel :type Integer))
  (returns (value :type "Float (double-precision)") (output :type Boolean))
  (locals (res :type "Float (double-precision)"))
  (bind _smoothlength (`self.Smoothlength`))
  (bind _output (`|GetArrayItem` (`self.nummemoarray`) channel))
  (bind _output_2 (`|GetArrayItem` (`self.memoarray`) channel))
  (bind _returnvalue (+ _output 1))
  (`|VariableSetRef` _output_2 (+ accvalue _output_2))
  (`|VariableSetRef` _output _returnvalue)
  (if (== _returnvalue _smoothlength)
    (bind _output_get (set `local.res` (/ (`|GetArrayItem` (`self.memoarray`) channel) _smoothlength)))
    (`|VariableSetRef` (`|GetArrayItem` (`self.memoarray`) channel))
    (`|VariableSetRef` (`|GetArrayItem` (`self.nummemoarray`) channel))
    (return _output_get true)
    (else
      (return -1.0 false))))

(fn `StartListenning`
  (`SynthComponent.Start` (`self.AudioCaptureComp`))
  (set `self.Listenning` true))

(fn `TriggerUIVisibilityEvent`
  (bind _asplayer_widget_1 (cast `/Game/UI/PlayerWidget1` (`WidgetComponent.GetUserWidgetObject` (`self.Widget`))))
  (if (== (`/Game/UI/PlayerWidget1.TableVisibility` _asplayer_widget_1) 2)
    (set `/Game/UI/PlayerWidget1.TableVisibility` "SelfHitTestInvisible" _asplayer_widget_1)
    (else
      (set `/Game/UI/PlayerWidget1.TableVisibility` "Hidden" _asplayer_widget_1))))

(fn `UserConstructionScript`)