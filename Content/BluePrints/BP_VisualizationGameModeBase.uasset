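; Game mode for an audio visualization level that runs audio buses and tracks music player positions.
; Every bus in AudioBusArray starts on BeginPlay and stops on EndPlay.
; Tick copies each MusicPlayerArray entry's sphere world location into the matching PlayerPostionArray slot.
; The code that finds MusicPlayer actors and fills both arrays is disconnected, and UpdatePositionInfo is an empty stub.
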(event `self.ReceiveBeginPlay`
  (for _array_element (`self.AudioBusArray`)
    (`AudioMixerBlueprintLibrary.StartAudioBus` _array_element)))

(event `self.ReceiveTick`
  (params (DeltaSeconds :type "Float (single-precision)"))
  (for (_array_element _array_index) (`self.MusicPlayerArray`)
    (`|VariableSetRef` (`|GetArrayItem` (`self.PlayerPostionArray`) _array_index) (`SceneComponent.K2_GetComponentLocation` (`/Game/BluePrints/MusicPlayer.Sphere` _array_element)))))

(event `self.ReceiveEndPlay`
  (params (EndPlayReason :type "EEndPlayReason Enum" :default "Destroyed"))
  (for _array_element (`self.AudioBusArray`)
    (`AudioMixerBlueprintLibrary.StopAudioBus` _array_element)))

(fn `UpdatePositionInfo`
  (locals (distanceMin2 :type "Vector Structure") (MaxRange :type "Float (double-precision)" :default 1000.0) (distanceMin1 :type "Vector Structure")))

(fn `UserConstructionScript`)