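; Wall actor whose material pulses with live audio, optionally applying a dynamic PulseWall material when UsePattern is set.
; BeginPlay starts submix spectral analysis; Tick averages clamped, power-compressed magnitudes at FreqArray frequencies from AudioSubmix into the material's "amp" parameter.
; SmoothValue is currently a pass-through, so no smoothing occurs.
; RadiusControlOld, an uncalled older path, drives "radius" from band-averaged Constant-Q NRT data.
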(event `self.ReceiveBeginPlay`
  (set `self.playtime` 0.0)
  (set `self.PatternRadius` 0.0)
  (`AudioMixerBlueprintLibrary.StartAnalyzingOutput` "/Game/Audio/Submix_Overall.Submix_Overall")
  (if (`self.UsePattern`)
    (bind _returnvalue (`PrimitiveComponent.CreateDynamicMaterialInstance` (`self.StaticMeshComponent`) 0 "/Game/Materials/PulseWall.PulseWall" "None"))
    (`PrimitiveComponent.SetMaterial` (`self.StaticMeshComponent`) 0 _returnvalue)))

(event `self.ReceiveTick`
  (params (DeltaSeconds :type "Float (single-precision)"))
  (bind _freqarray (`self.FreqArray`))
  (bind _magnitudes (`AudioMixerBlueprintLibrary.GetMagnitudeForFrequencies` _freqarray (`self.Audio Submix`)))
  (set `self.amp` 0.0)
  (for (_array_element _array_index) _magnitudes
    (bind _value (`self.Smooth Value` (`KismetMathLibrary.MultiplyMultiply_FloatFloat` (`KismetMathLibrary.FClamp` _array_element 0.0 1000.0) 0.3) _array_index))
    (set `self.amp` (+ _value (`self.amp`))))
  (`MeshComponent.SetScalarParameterValueOnMaterials` (`self.StaticMeshComponent`) "amp" (/ (`self.amp`) (`KismetArrayLibrary.Array_Length` _freqarray))))

(fn `Get Audio Strength`
  (params (time :type "Float (single-precision)") (BandsFilter :type "Vector2D Structure") (QNRT :type "ConstantQNRT Object Reference"))
  (returns (DeltaStrength :type "Float (double-precision)"))
  (locals (deltaQ :type "Float (double-precision)"))
  (bind (_x _y) (`KismetMathLibrary.BreakVector2D` BandsFilter))
  (set `local.deltaQ` (`self.AudioStrength`))
  (set `self.AudioStrength` 0.0)
  (for (_array_element _array_index) (`ConstantQNRT.GetNormalizedChannelConstantQAtTime` QNRT time 0)
    (if (`KismetMathLibrary.InRange_IntInt` _array_index (`KismetMathLibrary.FTrunc` _x) (`KismetMathLibrary.FTrunc` _y))
      (set `self.AudioStrength` (+ (`self.AudioStrength`) _array_element))))
  (bind _output_get (set `self.AudioStrength` (/ (`self.AudioStrength`) (- _y _x))))
  (`KismetSystemLibrary.PrintString` (`KismetStringLibrary.Conv_DoubleToString` _output_get) false false)
  (return (- (`local.deltaQ`) (`self.AudioStrength`))))

(fn `RadiusControlOld`
  (params (DeltaTime :type "Float (double-precision)"))
  (bind _output_get (set `self.playtime` (+ DeltaTime (`self.playtime`))))
  (bind _deltastrength (`self.Get Audio Strength` _output_get (`self.BandsFilter`) "/Game/Audio/ConstantAudioSynesthesiaNRT.ConstantAudioSynesthesiaNRT"))
  (`self.UpdatePatternRadius` _deltastrength DeltaTime)
  (`MeshComponent.SetScalarParameterValueOnMaterials` (`self.StaticMeshComponent`) "radius" (`self.AudioStrength`)))

(fn `Smooth Value`
  (params (accvalue :type "Float (double-precision)") (channel :type Integer))
  (returns (value :type "Float (double-precision)") (output :type Boolean))
  (return accvalue false))

(fn `UpdatePatternRadius`
  (params (DeltaStrength :type "Float (double-precision)") (DeltaTime :type "Float (double-precision)"))
  (if (< DeltaStrength 0.0)
    (set `self.PatternRadius` (- (`self.PatternRadius`) (* DeltaTime 1.5)))
    (else
      (set `self.PatternRadius` (+ (`self.PatternRadius`) DeltaTime))))
  (set `self.PatternRadius` (`KismetMathLibrary.FMin` (`self.PatternRadius`) 1.0)))

(fn `UserConstructionScript`)